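; Paper2D enemy character Zoro that chases the player and dies on taking any damage.
; Pawn sensing sets a seeing flag and triggers an AI MoveTo toward player zero; the flag is never cleared here.
; Any damage deactivates movement and plays the death flipbook.
; The hitbox is unhidden at start, but its overlap only casts to Luffy; the throttled damage logic is disconnected.
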(event `self.ReceiveBeginPlay`
  (`SceneComponent.SetHiddenInGame` (`self.Zoro_HitBox`) false false))

(event `self.ReceiveAnyDamage`
  (params (Damage :type "Float (single-precision)") (DamageType :type "DamageType Object Reference") (InstigatedBy :type "Controller Object Reference") (DamageCauser :type "Actor Object Reference"))
  (set `self.isDead` true)
  (`ActorComponent.SetActive` (`self.CharacterMovement`) false false)
  (`PaperFlipbookComponent.SetFlipbook` (`self.Sprite`) "/Game/CharacterArt/Zoro_Death.Zoro_Death"))

(event `self.Zoro_HitBox.OnComponentBeginOverlap`
  (params (OverlappedComponent :type "PrimitiveComponent Object Reference") (OtherActor :type "Actor Object Reference") (OtherComp :type "PrimitiveComponent Object Reference") (OtherBodyIndex :type Integer) (bFromSweep :type Boolean) (SweepResult :type "HitResult Structure (by ref)"))
  (bind _as2dcharacter_bp_luffy (cast `/Game/Blueprints/2DCharacter_BP_Luffy` OtherActor)))

(event `self.PawnSensing.OnSeePawn`
  (params (Pawn :type "Pawn Object Reference"))
  (set `self.isSeeingPlayer` true)
  (`self.FollowPlayer`))

(event `FollowPlayer`
  (if (`self.isSeeingPlayer`)
    (`|AIMoveTo` self (0.0 0.0 0.0) (`GameplayStatics.GetPlayerCharacter` 0))))

(fn `UserConstructionScript`)